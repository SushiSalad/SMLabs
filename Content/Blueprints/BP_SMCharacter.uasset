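; BP_SMCharacter is a character Blueprint that carries a rocket launcher, spawned on BeginPlay and attached to the mesh's right-hand socket.
; Tick derives Pitch from the first-person camera, and G toggles HoldingWeapon.
; Fire plays a montage and decrements the weapon's ammo, while R plays a montage and refills it to MaxAmmo.
; No projectile is spawned here, and neither montage call shows an assigned asset.
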(event `InputAction|Fire`
  (params (Key :type "Key Structure")))

(event `self.ReceiveTick`
  (params (DeltaSeconds :type "Float (single-precision)"))
  (set `self.pitch` (`.Pitch` (`KismetMathLibrary.GetYawPitchFromVector` (`SceneComponent.GetForwardVector` (`self.FPSCameraComponent`))))))

(event `Key|G`
  (params (Key :type "Key Structure"))
  (:`Pressed`
    (`/Engine/EditorBlueprintResources/StandardMacros.FlipFlop`
      (:`A`
        (set `self.holdingWeapon` true))
      (:`B`
        (set `self.holdingWeapon` false)))))

(event `self.ReceiveBeginPlay`
  (bind _returnvalue (`|SpawnActorFromClass` "/Game/Meshes/SMCharacter/Rocket_Launcher_BP.Rocket_Launcher_BP_C" (`KismetMathLibrary.MakeTransform` (0.0 0.0 0.0) (struct :`Pitch` -90.0) (0.2 0.2 0.2)) "Undefined" "OverrideRootScale" null null))
  (bind _output_get (set `self.weapon` _returnvalue))
  (`self.K2_AttachToComponent` _output_get (`self.Mesh`) "hand_rSocket" "KeepRelative" "KeepRelative" "KeepWorld" true))

(event `InputAction|Fire`
  (params (Key :type "Key Structure"))
  (:`Pressed`
    (bind _ammo (`/Game/Meshes/SMCharacter/Rocket_Launcher_BP.Ammo` (stale `self.ReceiveBeginPlay` _output_get)))
    (if (> _ammo 0)
      (bind _returnvalue (`self.PlayAnimMontage` null))
      (`KismetSystemLibrary.PrintString` (`KismetStringLibrary.Conv_DoubleToString` _returnvalue))
      (`/Engine/EditorBlueprintResources/StandardMacros.DecrementInt` _ammo))))

(event `Key|R`
  (params (Key :type "Key Structure"))
  (:`Pressed`
    (bind _max_ammo (`/Game/Meshes/SMCharacter/Rocket_Launcher_BP.Max_Ammo` (stale `self.ReceiveBeginPlay` _output_get)))
    (if (< (`/Game/Meshes/SMCharacter/Rocket_Launcher_BP.Ammo` (stale `self.ReceiveBeginPlay` _output_get)) _max_ammo)
      (`self.PlayAnimMontage` null)
      (set `/Game/Meshes/SMCharacter/Rocket_Launcher_BP.Ammo` _max_ammo (stale `self.ReceiveBeginPlay` _output_get)))))

(fn `UserConstructionScript`)
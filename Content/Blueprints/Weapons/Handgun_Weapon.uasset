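; Handgun weapon Blueprint that plays the gun's fire and reload animations.
; OnFire and OnReload each play a one-shot animation on the Handgun skeletal mesh.
; The construction script fills Ammo to MaxAmmo, assigns the mesh to SkeleMesh and stores the character fire and reload montages in an array.
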(event `self.onFire`
  (`SkeletalMeshComponent.PlayAnimation` (`self.Handgun`) "/Game/Animations/Weapon/handgun_fire.handgun_fire" false))

(event `self.onReload`
  (`SkeletalMeshComponent.PlayAnimation` (`self.Handgun`) "/Game/Animations/Weapon/handgun_reload.handgun_reload" false))

(fn `UserConstructionScript`
  (set `self.ammo` (`self.maxAmmo`))
  (set `self.skeleMesh` (`self.Handgun`))
  (set `self.montage` (`|MakeArray` "/Game/Animations/Character/character_handgun_fire_anim_Montage.character_handgun_fire_anim_Montage" "/Game/Animations/Character/character_handgun_reload_anim_character_characterAction_Montage.character_handgun_reload_anim_character_characterAction_Montage" :!type "AnimMontage Object Reference")))
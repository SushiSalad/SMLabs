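; Rocket launcher weapon Blueprint that configures a single-round weapon through its stats and assets.
; The construction script sets ammo, spread, fire rate, damage, reload speed and weight, plus the launcher skeletal mesh and character fire and reload montages.
; The event graph holds only leftover test nodes: a "Hello" print handler for OnFire, with its binding and a Fire call both unconnected.
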(event `onFire_Event_0`
  (`KismetSystemLibrary.PrintString` "Hello"))

(fn `UserConstructionScript`
  (bind _output_get (set `self.maxAmmo` 1))
  (set `self.ammo` _output_get)
  (set `self.bulletSpread` 10)
  (set `self.fireRate` 100)
  (set `self.damage` 20)
  (set `self.reloadSpeed` 2)
  (set `self.weight` 10)
  (set `self.skeleMesh` (`self.RocketLauncher`))
  (set `self.montage` (`|MakeArray` "/Game/Animations/Character/character_rocket_fire_anim_Montage.character_rocket_fire_anim_Montage" "/Game/Animations/Character/character_rocket_reload_anim_Montage.character_rocket_reload_anim_Montage" :!type "AnimMontage Object Reference")))
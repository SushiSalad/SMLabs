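; BP_SMCharacter is a first-person character that carries a rocket launcher and respawns after death.
; BeginPlay attaches the launcher to the right hand; Fire plays a montage and spends ammo, while R only plays a reload montage, as the refill is unconnected.
; Tick stores camera pitch, and G toggles IsHoldingWeapon.
; Lethal damage sets IsDead, waits, then moves the character to a random Team1Spawn PlayerStart and restores health.
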(event `self.ReceiveTick`
  (params (DeltaSeconds :type "Float (single-precision)"))
  ;[1 1 1] Get Camera Pitch
  (set `self.pitch` (`.Pitch` (`KismetMathLibrary.GetYawPitchFromVector` (`SceneComponent.GetForwardVector` (`self.FPSCameraComponent`))))))

(event `Key|G`
  (params (Key :type "Key Structure"))
  ;[1 1 1] Holster Weapon
  (:`Pressed`
    (`/Engine/EditorBlueprintResources/StandardMacros.FlipFlop`
      (:`A`
        (set `self.isHoldingWeapon` true))
      (:`B`
        (set `self.isHoldingWeapon` false)))))

(event `InputAction|Fire`
  (params (Key :type "Key Structure"))
  ;[1 1 1] Weapon Stuff
  (:`Pressed`
    (bind _ammo (`/Game/Meshes/SMCharacter/Rocket_Launcher_BP.Ammo` (stale `self.ReceiveBeginPlay` _output_get)))
    (if (> _ammo 0)
      (bind _returnvalue (`self.PlayAnimMontage` "/Game/Animations/Character/character_rocket_fire_anim_Montage.character_rocket_fire_anim_Montage"))
      (`KismetSystemLibrary.PrintString` (`KismetStringLibrary.Conv_DoubleToString` _returnvalue))
      (`/Engine/EditorBlueprintResources/StandardMacros.DecrementInt` _ammo))))

(event `self.ReceiveBeginPlay`
  ;[1 1 1] Weapon Stuff
  (bind _returnvalue (`|SpawnActorFromClass` "/Game/Meshes/SMCharacter/Rocket_Launcher_BP.Rocket_Launcher_BP_C" (`KismetMathLibrary.MakeTransform` (0.0 0.0 0.0) (struct :`Pitch` -90.0) (0.2 0.2 0.2)) "Undefined" "OverrideRootScale" null null))
  (bind _output_get (set `self.weapon` _returnvalue))
  (`self.K2_AttachToComponent` _output_get (`self.Mesh`) "hand_rSocket" "KeepRelative" "KeepRelative" "KeepWorld" true))

(event `Key|R`
  (params (Key :type "Key Structure"))
  ;[1 1 1] Weapon Stuff
  (:`Pressed`
    (if (< 0 (`/Game/Meshes/SMCharacter/Rocket_Launcher_BP.Max_Ammo` (stale `self.ReceiveBeginPlay` _output_get)))
      (`self.PlayAnimMontage` "/Game/Animations/Character/character_rocket_reload_anim_Montage.character_rocket_reload_anim_Montage"))))

(event `self.ReceiveAnyDamage`
  (params (Damage :type "Float (single-precision)") (DamageType :type "DamageType Object Reference") (InstigatedBy :type "Controller Object Reference") (DamageCauser :type "Actor Object Reference"))
  ;[1 1 1] Take damage and respawn player
  (bind _output_get (set `self.health` (- (`self.health`) Damage)))
  (if (<= _output_get 0.0)
    (set `self.isDead` true)
    (`KismetSystemLibrary.Delay` (`self.respawnDelay`))
    (set `self.isDead` false)
    (bind _outactors (`GameplayStatics.GetAllActorsOfClassWithTag` "/Script/Engine.PlayerStart" "Team1Spawn"))
    (bind _spawnvector (`self.Spawn Vector from Player Start Array` _outactors))
    (`self.K2_SetActorLocation` _spawnvector)
    (set `self.health` 100.0)))

(fn `Spawn Vector from Player Start Array`
  (params (actorArray :type "Array of Actor Object Reference"))
  (returns (spawnVector :type "Vector Structure"))
  (return (`self.K2_GetActorLocation` (`|GetArrayItem` actorArray (`KismetMathLibrary.RandomInteger` (`KismetArrayLibrary.Array_Length` actorArray))))))

(fn `UserConstructionScript`)